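; Player controller for the shooting game that passes the player's locally stored name to their player state when a pawn is possessed.
; On possession, the server notifies the client, which reads the name from ShootingGameInstance and sends it back through ReqSetNewName.
; The server then applies it with SetName on BP_ShootingPlayerState, completing a server-client-server round trip.
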(event `ResClientPossess`
  ;[1 1 1] (Client) 빙의 이벤트 수신
  (`KismetSystemLibrary.PrintString` (`KismetStringLibrary.Concat_StrStr` "ResClientPossess - " (`KismetSystemLibrary.GetDisplayName` self)) false false (struct :`G` 0.66 :`B` 1.0 :`A` 1.0) 60.0)
  (bind _asshooting_game_instance (cast `/Game/Shooting/GameMode/ShootingGameInstance` (`GameplayStatics.GetGameInstance`)))
  (`self.ReqSetNewName` (`/Game/Shooting/GameMode/ShootingGameInstance.Name` _asshooting_game_instance)))

(event `self.ReceivePossess`
  (params (PossessedPawn :type "Pawn Object Reference"))
  ;[1 0 0] (Server) 빙의 이벤트
  (`KismetSystemLibrary.PrintString` (`KismetStringLibrary.Concat_StrStr` "OnPossess - " (`KismetSystemLibrary.GetDisplayName` PossessedPawn)) false false (struct :`G` 0.66 :`B` 1.0 :`A` 1.0) 60.0)
  (`self.ResClientPossess`))

(event `ReqSetNewName`
  (params (NewName :type String))
  ;[1 0 0] (Server) 새로운 이름 적용
  (`KismetSystemLibrary.PrintString` "ReqSetNewName" true true (struct :`G` 0.66 :`B` 1.0 :`A` 1.0) 60.0)
  (bind _asbp_shooting_player_state (cast `/Game/Shooting/GameMode/BP_ShootingPlayerState` (`self.PlayerState`)))
  (`/Game/Shooting/GameMode/BP_ShootingPlayerState.SetName` _asbp_shooting_player_state NewName))

(fn `UserConstructionScript`)