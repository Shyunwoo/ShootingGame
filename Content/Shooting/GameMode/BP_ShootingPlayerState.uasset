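; BP_ShootingPlayerState is the shooting mode's player state, holding replicated health, name and kill count.
; Setter functions change these values, with health clamped to 0–100 and AddDamage returning whether the hit was lethal.
; OnRep handlers broadcast event dispatchers, plus a HUD-specific health one when this state belongs to player controller 0.
; On BeginPlay it binds itself to BP_ShootingHud, retrying on a short timer until that HUD exists.
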(event `self.ReceiveBeginPlay`
  (`self.InitBindHud`))

(fn `AddDamage`
  (params (Damage :type "Float (double-precision)"))
  (returns (IsKill :type Boolean))
  (if (> (`self.Hp`) 0.0)
    (bind _output_get (set `self.Hp` (`KismetMathLibrary.FClamp` (- (`self.Hp`) Damage) 0.0 100.0)))
    (return (<= _output_get 0.0))
    (else
      (return false))))

(fn `AddHeal`
  (params (HealValue :type "Float (double-precision)"))
  (set `self.Hp` (`KismetMathLibrary.FClamp` (+ (`self.Hp`) HealValue) 0.0 100.0)))

(fn `AddKillCount`
  (set `self.KillCount` (+ (`self.KillCount`) 1)))

(fn `InitBindHud`
  (bind _asbp_shooting_hud (cast `/Game/Shooting/GameMode/BP_ShootingHud` (`PlayerController.GetHUD` (`GameplayStatics.GetPlayerController` 0)))
    (:`then`
      (`/Game/Shooting/GameMode/BP_ShootingHud.BindPlayerState` _asbp_shooting_hud self))
    (:`CastFailed`
      (`KismetSystemLibrary.K2_SetTimer` null "InitBindHud" 0.1))))

(fn `OnRep_Hp`
  (`KismetSystemLibrary.PrintString` (`KismetStringLibrary.Concat_StrStr` "OnRepHp CurHP - " (`KismetStringLibrary.Conv_DoubleToString` (`self.Hp`))) false false (struct :`G` 0.66 :`B` 1.0 :`A` 1.0) 20.0)
  (`self.EventDispatcher_UpdateHp` (`self.Hp`) 100.0)
  (if (== (`Controller.PlayerState` (`GameplayStatics.GetPlayerController` 0)) self)
    (`self.EventDispatcher_UpdateHpHUD` (`self.Hp`) 100.0)))

(fn `OnRep_KillCount`
  (`KismetSystemLibrary.PrintString` (`KismetStringLibrary.Concat_StrStr` "On Rep Kill Count Name  - " (`self.Name`) ", Kill Count - " (`KismetStringLibrary.Conv_IntToString` (`self.KillCount`))) false false (struct :`G` 0.66 :`B` 1.0 :`A` 1.0) 60.0)
  (`self.EventDispatcher_KillCount` (`self.KillCount`)))

(fn `OnRep_Name`
  (`KismetSystemLibrary.PrintString` (`KismetStringLibrary.Concat_StrStr` "OnRepName - " (`self.Name`)) true true (struct :`G` 0.66 :`B` 1.0 :`A` 1.0) 60.0)
  (`self.EventDispatcher_ChangeName` (`self.Name`)))

(fn `SetName`
  (params (Name :type String))
  (set `self.Name` Name))

(fn `UserConstructionScript`)