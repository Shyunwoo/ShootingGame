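; BP_ShootingHud is the shooting game's HUD, creating the main HUD widget on BeginPlay and switching to game-only input without a cursor.
; It forwards ammo, HP, kill-list refreshes and Enter-key text entry to that widget.
; HP and kill-count events bind to player state dispatchers.
; Short function-name timers retry until the local player state exists for HP binding and the widget is valid for the kill-list refresh.
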(event `self.ReceiveBeginPlay`
  (bind _returnvalue (`GameplayStatics.GetPlayerController` 0))
  (bind _returnvalue_2 (`|CreateWidget` "/Game/Shooting/Widget/ShootingHudWidget.ShootingHudWidget_C"))
  (bind _output_get (set `self.HudWidget` _returnvalue_2))
  (`UserWidget.AddToViewport` _output_get 0)
  (`self.UpdateBindPlayerState`)
  (`WidgetBlueprintLibrary.SetInputMode_GameOnly` _returnvalue)
  (set `PlayerController.bShowMouseCursor` false _returnvalue))

(fn `BindPlayerState`
  (params (PlayerState :type "/Game/Shooting/GameMode/BP_ShootingPlayerState Object Reference"))
  (add `/Game/Shooting/GameMode/BP_ShootingPlayerState.EventDispatcher_KillCount` PlayerState (`|CreateDelegate` :!event `UpdateKillCount`))
  (`self.UpdateKillCountWithBind`))

(fn `PressEnter`
  (`/Game/Shooting/Widget/ShootingHudWidget.ShowEditText` (`self.HudWidget`)))

(fn `SetAmmoText`
  (params (Ammo :type Integer))
  (`/Game/Shooting/Widget/ShootingHudWidget.SetAmmoText` (`self.HudWidget`) Ammo))

(fn `SetHp`
  (params (CurHp :type "Float (double-precision)") (MaxHp :type "Float (double-precision)"))
  (`/Game/Shooting/Widget/ShootingHudWidget.SetHP` (`self.HudWidget`) CurHp MaxHp))

(fn `UpdateBindPlayerState`
  (bind _asbp_shooting_player_state (cast `/Game/Shooting/GameMode/BP_ShootingPlayerState` (`Controller.PlayerState` (`GameplayStatics.GetPlayerController` 0)))
    (:`then`
      (add `/Game/Shooting/GameMode/BP_ShootingPlayerState.EventDispatcher_UpdateHpHUD` _asbp_shooting_player_state (`|CreateDelegate` :!event `SetHp`)))
    (:`CastFailed`
      (`KismetSystemLibrary.K2_SetTimer` null "UpdateBindPlayerState" 0.1))))

(fn `UpdateKillCount`
  (params (KillCount :type Integer))
  (`KismetSystemLibrary.PrintString` (`KismetStringLibrary.Concat_StrStr` "Update Kill Count - " (`KismetStringLibrary.Conv_IntToString` KillCount)) true true (struct :`G` 0.66 :`B` 1.0 :`A` 1.0) 60.0)
  (`/Game/Shooting/Widget/ShootingHudWidget.UpdateKillCountList` (`self.HudWidget`)))

(fn `UpdateKillCountWithBind`
  (bind _hudwidget (`self.HudWidget`))
  (`/Engine/EditorBlueprintResources/StandardMacros.IsValid` _hudwidget
    (:`Is Valid`
      (`/Game/Shooting/Widget/ShootingHudWidget.UpdateKillCountList` _hudwidget))
    (:`Is Not Valid`
      (`KismetSystemLibrary.K2_SetTimer` null "UpdateKillCountWithBind" 0.1))))

(fn `UserConstructionScript`)