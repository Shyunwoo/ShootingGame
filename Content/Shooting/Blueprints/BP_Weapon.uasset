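; Networked weapon actor for a shooting game, configured by name from DT_Weapon and attachable to or droppable from a character's mesh socket.
; Trigger and reload play montages; separate shoot and reload functions handle effects, hit checks and refills, with ammo shown on the local HUD.
; The owning client line-traces from the camera and requests damage from the server.
; BP_Rock hits instead break the mesh via a client event, then destroy it after a delay.
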(event `self.ReceiveBeginPlay`
  (`self.Initialize`))

(event `ResDestructible`
  (params (DamagedActor :type "Actor Object Reference (by ref)") (Location :type "Vector Structure") (ImpactPoint :type "Vector Structure"))
  ;[1 1 1] (Clinet)
  (bind _asbp_rock (cast `/Game/Shooting/Blueprints/BP_Rock` DamagedActor))
  (`/Game/Shooting/Blueprints/BP_Rock.DoDestructMesh` _asbp_rock Location ImpactPoint))

(event `ReqApplyDamage`
  (params (DamagedActor :type "Actor Object Reference (by ref)") (BaseDamage :type "Float (double-precision)") (EventInstigator :type "Controller Object Reference (by ref)") (DamageCauser :type "Actor Object Reference (by ref)") (Location :type "Vector Structure") (ImpactPoint :type "Vector Structure"))
  ;[1 0 0] (Server)
  (bind _asbp_rock (cast `/Game/Shooting/Blueprints/BP_Rock` DamagedActor)
    (:`then`
      (`self.ResDestructible` _asbp_rock Location ImpactPoint)
      (`KismetSystemLibrary.Delay` 5.0)
      (`/Game/Shooting/Blueprints/BP_Rock.DoDestroy` _asbp_rock))
    (:`CastFailed`
      (`GameplayStatics.ApplyDamage` DamagedActor BaseDamage EventInstigator DamageCauser)
      (`KismetSystemLibrary.PrintString` (`KismetStringLibrary.Concat_StrStr` "(Server) ApplyDamage - " (`KismetSystemLibrary.GetDisplayName` DamagedActor)) false false (struct :`R` 1.0 :`A` 1.0) 20.0))))

(fn `AttachToChar`
  (params (Character :type "Character Object Reference"))
  (returns (Result :type Boolean) (Actor :type "Actor Object Reference"))
  (bind _staticmesh (`self.StaticMesh`))
  (bind _output_get (set `self.OwnChar` Character))
  (`PrimitiveComponent.SetSimulatePhysics` _staticmesh false)
  (`PrimitiveComponent.SetCollisionEnabled` _staticmesh "NoCollision")
  (bind _returnvalue (`SceneComponent.K2_AttachToComponent` _staticmesh (`Character.Mesh` _output_get) (`self.Socket Name`) "SnapToTarget" "SnapToTarget" "KeepWorld" true))
  (`|ExecutionSequence`
    (:`then_0`
      (if (== (`self.OwnChar`) (`GameplayStatics.GetPlayerCharacter` 0))
        (bind _asbp_shooting_hud (cast `/Game/Shooting/GameMode/BP_ShootingHud` (`PlayerController.GetHUD` (`GameplayStatics.GetPlayerController` 0))))
        (`/Game/Shooting/GameMode/BP_ShootingHud.SetAmmoText` _asbp_shooting_hud (`self.CurAmmo`))))
    (:`then_1`
      (return _returnvalue self))))

(fn `CheckShootable`
  (returns (Shootable :type Boolean))
  (`/Engine/EditorBlueprintResources/StandardMacros.IsValid` (`self.OwnChar`)
    (:`Is Valid`
      (if (> (`self.CurAmmo`) 0)
        (return true)
        (else
          (return false))))
    (:`Is Not Valid`
      (return false))))

(fn `DetachToChar`
  (params (Character :type "Character Object Reference"))
  (returns (Result :type Boolean))
  (bind _staticmesh (`self.StaticMesh`))
  (set `self.OwnChar` null)
  (`self.SetOwner` null)
  (`PrimitiveComponent.SetCollisionEnabled` _staticmesh "QueryAndPhysics")
  (`PrimitiveComponent.SetSimulatePhysics` _staticmesh true)
  (`SceneComponent.K2_DetachFromComponent` _staticmesh "KeepWorld" "KeepWorld" "KeepWorld" true)
  (return true))

(fn `DoReload`
  (params (Character :type "Character Object Reference"))
  (returns (Result :type Boolean))
  (bind _output_get (set `self.CurAmmo` (`.Ammo_11_6838F29C469296FC38997283F52A2ED3` (break `/Game/Shooting/Data/ST_Weapon` (`self.WeaponData`)))))
  (if (== (`self.OwnChar`) (`GameplayStatics.GetPlayerCharacter` 0))
    (bind _asbp_shooting_hud (cast `/Game/Shooting/GameMode/BP_ShootingHud` (`PlayerController.GetHUD` (`GameplayStatics.GetPlayerController` 0))))
    (`/Game/Shooting/GameMode/BP_ShootingHud.SetAmmoText` _asbp_shooting_hud _output_get)
    (return true)
    (else
      (return true))))

(fn `DoShoot`
  (params (Character :type "Character Object Reference"))
  (returns (Result :type Boolean))
  (bind _returnvalue (`GameplayStatics.GetPlayerCameraManager` 0))
  (bind _audio (`self.Audio`))
  (bind _returnvalue_2 (`self.K2_GetActorLocation` _returnvalue))
  (`AudioComponent.SetSound` _audio (`.ShootSound_6_64EF1271444D804A6D0E0683ED5F7091` (break `/Game/Shooting/Data/ST_Weapon` (`self.WeaponData`))))
  (`AudioComponent.Play` _audio 0.0)
  (`GameplayStatics.SpawnEmitterAtLocation` "/Game/StarterContent/Particles/P_Explosion.P_Explosion" (`SceneComponent.GetSocketLocation` (`self.StaticMesh`) "Muzzle") (struct) (0.1 0.1 0.1))
  ;[1 1 1] 소유한 클라이언트에서 히트 채크
  (if (== (`self.OwnChar`) (`GameplayStatics.GetPlayerPawn` 0))
    (bind (_outhit _returnvalue_3) (`KismetSystemLibrary.LineTraceSingleForObjects` (+ _returnvalue_2 (* (`self.GetActorForwardVector` _returnvalue) 350.0)) (+ _returnvalue_2 (* (`self.GetActorForwardVector` _returnvalue) 10000.0)) (`|MakeArray` "ObjectTypeQuery1" "ObjectTypeQuery2" "ObjectTypeQuery3" "ObjectTypeQuery4" "ObjectTypeQuery6" :!type "EObjectTypeQuery Enum")))
    (if _returnvalue_3
      (`KismetSystemLibrary.PrintString` "(Client) ReqApplyDamage" false false (struct :`G` 0.66 :`B` 1.0 :`A` 1.0) 20.0)
      (bind (_bblockinghit _binitialoverlap _time _distance _location _impactpoint _normal _impactnormal _physmat _hitactor) (`GameplayStatics.BreakHitResult` _outhit))
      (`self.ReqApplyDamage` _hitactor 10.0 (`Pawn.GetController` (`self.OwnChar`)) self _location _impactpoint)
      (return true))))

(fn `Initialize`
  (bind _returnvalue (`|GetDataTableRow` "/Game/Shooting/Data/DT_Weapon.DT_Weapon" (`self.WeaponName`))
    (:`then`
      (bind _output_get (set `self.WeaponData` _returnvalue))
      (`|ExecutionSequence`
        (:`then_0`
          (bind (_staticmesh _socketname _shootsound _reloadsound _ammo) (break `/Game/Shooting/Data/ST_Weapon` _output_get))
          (`StaticMeshComponent.SetStaticMesh` (`self.StaticMesh`) _staticmesh))
        (:`then_1`
          (set `self.Socket Name` _socketname))
        (:`then_2`
          (set `self.CurAmmo` _ammo))))))

(fn `PlayReloadAnim`
  (params (Character :type "Character Object Reference"))
  (returns (Result :type Boolean))
  (bind _ownchar (`self.OwnChar`))
  (bind (_staticmesh _socketname _shootsound _reloadsound _ammo _shootmontage _shootmontageplayrate _reloadmontage _reloadmontageplayrate) (break `/Game/Shooting/Data/ST_Weapon` (`self.WeaponData`)))
  (`/Engine/EditorBlueprintResources/StandardMacros.IsValid` _ownchar
    (:`Is Valid`
      (`AnimInstance.Montage_Play` (`SkeletalMeshComponent.GetAnimInstance` (`Character.Mesh` _ownchar)) _reloadmontage _reloadmontageplayrate "MontageLength" 0.0 true)
      (return false))))

(fn `PlayShootMontage`
  (bind _ownchar (`self.OwnChar`))
  (bind (_staticmesh _socketname _shootsound _reloadsound _ammo _shootmontage _shootmontageplayrate) (break `/Game/Shooting/Data/ST_Weapon` (`self.WeaponData`)))
  (bind _shootable (`self.CheckShootable`))
  (if _shootable
    (`/Engine/EditorBlueprintResources/StandardMacros.IsValid` _ownchar
      (:`Is Valid`
        (`AnimInstance.Montage_Play` (`SkeletalMeshComponent.GetAnimInstance` (`Character.Mesh` _ownchar)) _shootmontage _shootmontageplayrate "MontageLength" 0.0 true)
        (bind _result (`/Engine/EditorBlueprintResources/StandardMacros.DecrementInt` (`self.CurAmmo`))
          (:`  `
            (if (== (`self.OwnChar`) (`GameplayStatics.GetPlayerCharacter` 0))
              (bind _asbp_shooting_hud (cast `/Game/Shooting/GameMode/BP_ShootingHud` (`PlayerController.GetHUD` (`GameplayStatics.GetPlayerController` 0))))
              (`/Game/Shooting/GameMode/BP_ShootingHud.SetAmmoText` _asbp_shooting_hud _result))))))))

(fn `PullTrigger`
  (params (Character :type "Character Object Reference"))
  (returns (Result :type Boolean))
  (`self.PlayShootMontage`)
  (return true))

(fn `ReleaseTrigger`
  (params (Character :type "Character Object Reference"))
  (returns (Result :type Boolean))
  (return false))

(fn `UserConstructionScript`)