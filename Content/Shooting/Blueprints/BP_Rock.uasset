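; BP_Rock is a destructible rock actor that can be shattered by a hit or removed from the world.
; DoDestructMesh stores the hit location and impulse direction, then sets IsDestruct, whose RepNotify applies heavy damage and impulse to the Destructible component.
; DoDestroy sets IsDestroyed, whose RepNotify destroys the actor.
; Both effects are driven by replicated state, with no direct RPCs in the graphs.
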(fn `DoDestroy`
  (set `self.IsDestroyed` true))

(fn `DoDestructMesh`
  (params (HitLocation :type "Vector Structure (by ref)") (ImpulseDir :type "Vector Structure (by ref)"))
  (set `self.Hit Location` HitLocation)
  (set `self.Impulse Dir` ImpulseDir)
  (set `self.IsDestruct` true))

(fn `OnRep_IsDestroyed`
  (if (`self.IsDestroyed`)
    (`self.K2_DestroyActor`)))

(fn `OnRep_IsDestruct`
  (`DestructibleComponent.ApplyDamage` (`self.Destructible`) 10000.0 (`self.Hit Location`) (`self.Impulse Dir`) 10000.0))

(fn `UserConstructionScript`)